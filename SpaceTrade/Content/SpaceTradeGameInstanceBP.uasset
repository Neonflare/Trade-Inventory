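; Game instance for the space trade game that drives top-level switching between the main menu and gameplay through a state machine.
; Init sets up the state machine, binds StateChanged and enters MainMenu.
; Each handled state opens its level, waits briefly, then shows a lazily created, cached widget with the mouse cursor visible.
; The menu also unpauses and uses UI-only input, while In Game clears existing widgets first and shows InventoryTest.
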(event `self.ReceiveInit`
  (bind _statemachine (`self.StateMachine`))
  (set `MenuStateMachine.States` (`self.InitialState`) _statemachine)
  (add `MenuStateMachine.OnStateChanged` _statemachine (delegate `StateChanged`))
  (`MenuStateMachine.SetState` _statemachine "MainMenu"))

(event `StateChanged`
  (params (NewState :type String) (OldState :type String))
  (bind _returnvalue (`GameplayStatics.GetPlayerController` 0))
  (bind _mainmenu (`self.MainMenu`))
  (switch `string` NewState
    (:`MainMenu`
      (switch `string` OldState
        (:``
          _)
        (:`InGame`
          _)
        (:`Options`
          _))
      (`GameplayStatics.OpenLevel` "MainMenu")
      (`KismetSystemLibrary.Delay` 0.2)
      (`GameplayStatics.SetGamePaused` false)
      (if (not (`KismetSystemLibrary.IsValid` (`self.MainMenu`)))
        (bind _returnvalue_2 (`|CreateWidget` "/Game/MainMenuScreen.MainMenuScreen_C"))
        (set `self.MainMenu` _returnvalue_2))
      (`UserWidget.AddToViewport` _mainmenu 0)
      (`WidgetBlueprintLibrary.SetInputMode_UIOnlyEx` _returnvalue _mainmenu)
      (set `PlayerController.bShowMouseCursor` true _returnvalue))
    (:`InGame`
      (`WidgetLayoutLibrary.RemoveAllWidgets`)
      (`GameplayStatics.OpenLevel` "SpaceTradeGameScreen")
      (`KismetSystemLibrary.Delay` 0.2)
      (if (not (`KismetSystemLibrary.IsValid` (`self.Inventory Test`)))
        (bind _returnvalue_3 (`|CreateWidget` "/Game/InventoryTest.InventoryTest_C"))
        (set `self.Inventory Test` _returnvalue_3))
      (`UserWidget.AddToViewport` (`self.Inventory Test`) 0)
      (set `PlayerController.bShowMouseCursor` true (`GameplayStatics.GetPlayerController` 0)))))